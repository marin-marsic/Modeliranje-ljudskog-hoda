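; CameraBP is an actor, apparently a camera rig, that travels along its Path spline.
; Each Tick grows CurrDistance by an FInterpTo result with no Current input, so the step scales with spline length, Speed and delta time rather than easing toward the end.
; The Capsule then takes the spline's world location and rotation at that distance, without sweep.
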(event EventBeginPlay)

(event EventActorBeginOverlap
  (params (OtherActor :type Actor%20Object%20Reference)))

(event EventTick
  (params (DeltaSeconds :type Float%20%28single-precision%29))
  (bind _path (Variables|Default|GetPath))
  (bind _output_get (Variables|Default|SetCurrDistance (+ (stale _output_get) (Math|Interpolation|FInterpTo 0.0 (Spline|GetSplineLength (Variables|Default|GetPath)) DeltaSeconds (Variables|Default|GetSpeed)))))
  (Transformation|SetWorldLocationAndRotation (Variables|Default|GetCapsule) (Class|SplineComponent|GetWorldLocationatDistanceAlongSpline _path _output_get) (Class|SplineComponent|GetWorldRotationatDistanceAlongSpline _path _output_get) false))

(fn ConstructionScript)